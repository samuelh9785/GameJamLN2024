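; Behavior tree task that sends a BP_Ennemy back to the center of its search area when it strays too far.
; If its distance from the center reaches search radius plus max follow radius, it resets the iteration counter and player-seen blackboard flags, then moves there with AI Move To.
; It finishes successfully on arrival, or immediately if still in range; a failed move has no finish handler.
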(event `self.ReceiveExecuteAI`
  (params (OwnerController :type "AIController Object Reference") (ControlledPawn :type "Pawn Object Reference"))
  (bind _blackboard (`self.BlackBoard`))
  (set `self.Controlled Pawn` ControlledPawn)
  (set `self.BlackBoard` (`AIBlueprintHelperLibrary.GetBlackboard` (`AIBlueprintHelperLibrary.GetAIController` ControlledPawn)))
  (bind _asbp_ennemy (cast `/Game/_GameJamLN2024/Blueprints/Ennemy/BP_Ennemy` (`self.Controlled Pawn`)))
  (bind _searchareacenter (`/Game/_GameJamLN2024/Blueprints/Ennemy/BP_Ennemy.SearchAreaCenter` _asbp_ennemy))
  (set `self.Search Area Center` _searchareacenter)
  (if (>= (`KismetMathLibrary.Vector_Distance` _searchareacenter (`Actor.K2_GetActorLocation` _asbp_ennemy)) (+ (`/Game/_GameJamLN2024/Blueprints/Ennemy/BP_Ennemy.SearchRadius` _asbp_ennemy) (`/Game/_GameJamLN2024/Blueprints/Ennemy/BP_Ennemy.FollowPlayerMaxRadius` _asbp_ennemy)))
    (`BlackboardComponent.SetValueAsInt` _blackboard (`self.NbIterationName`) 0)
    (`BlackboardComponent.SetValueAsBool` _blackboard (`self.HasSeenPlayerName`) false)
    (`BlackboardComponent.SetValueAsBool` _blackboard (`self.CanSeePlayerName`) false)
    (`|AIMoveTo` (`self.Controlled Pawn`) (`self.Search Area Center`) null 50.0
      (:`OnSuccess`
        (`self.FinishExecute` true)))
    (else
      (`self.FinishExecute` true))))