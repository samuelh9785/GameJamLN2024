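; Behavior tree task that makes an enemy search for the player around the last seen location.
; Each run increments a Blackboard counter, moves to that location, then overwrites it with a random reachable point nearby for the next run.
; Once the counter exceeds the maximum, it resets the counter and clears the has-seen and can-see player flags.
; A failed move never finishes the task, as only success is handled.
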(event `self.ReceiveExecuteAI`
  (params (OwnerController :type "AIController Object Reference") (ControlledPawn :type "Pawn Object Reference"))
  (bind _blackboard (`self.BlackBoard`))
  (bind _returnvalue (`BlackboardComponent.GetValueAsVector` (`self.BlackBoard`) (`self.LastSeenPlayerLocationName`)))
  (bind _returnvalue_2 (`BlackboardComponent.GetValueAsInt` (`self.BlackBoard`) (`self.NbIterationName`)))
  (set `self.Controlled Pawn` ControlledPawn)
  (set `self.BlackBoard` (`AIBlueprintHelperLibrary.GetBlackboard` (`AIBlueprintHelperLibrary.GetAIController` ControlledPawn)))
  (if (<= _returnvalue_2 (`self.NbMaxIteration`))
    (bind _result (`/Engine/EditorBlueprintResources/StandardMacros.IncrementInt` _returnvalue_2)
      (:`  `
        (`BlackboardComponent.SetValueAsInt` (`self.BlackBoard`) (`self.NbIterationName`) _result)
        (`|AIMoveTo` (`self.Controlled Pawn`) _returnvalue null 100.0
          (:`OnSuccess`
            (`BlackboardComponent.SetValueAsVector` (`self.BlackBoard`) (`self.LastSeenPlayerLocationName`) (`NavigationSystemV1.K2_GetRandomReachablePointInRadius` _returnvalue (`self.Radius`) null null))
            (`self.FinishExecute` true)))))
    (else
      (`BlackboardComponent.SetValueAsInt` _blackboard (`self.NbIterationName`) 0)
      (`BlackboardComponent.SetValueAsBool` _blackboard (`self.HasSeenPlayerName`) false)
      (`BlackboardComponent.SetValueAsBool` _blackboard (`self.CanSeePlayerName`) false)
      (`self.FinishExecute` true))))