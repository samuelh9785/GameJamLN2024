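; Enemy girl AI character that searches around its start location, detects the player through AI Perception, and resets the game on contact.
; Perception updates write can-see, has-seen and last-seen-location keys to the AI controller's blackboard.
; A capsule hit with BP_Character calls Reset on BP_GameMode, while the enemy's own Reset teleports it home and clears the sight flags.
; The construction script draws debug circles previewing search and follow radii.
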(event `self.ReceiveBeginPlay`
  (set `self.SearchAreaCenter` (`self.K2_GetActorLocation`)))

(event `self.AIPerception.OnTargetPerceptionUpdated`
  (params (Actor :type "Actor Object Reference") (Stimulus :type "AIStimulus Structure"))
  (bind _canseeplayername (`self.CanSeePlayerName`))
  (bind _returnvalue (`AIBlueprintHelperLibrary.GetBlackboard` (`AIBlueprintHelperLibrary.GetAIController` self)))
  (if Stimulus_bSuccessfullySensed
    (cast `/Game/_GameJamLN2024/Blueprints/Player/BP_Character` Actor)
    (`KismetSystemLibrary.PrintString` "See character")
    (`BlackboardComponent.SetValueAsBool` _returnvalue _canseeplayername true)
    (`BlackboardComponent.SetValueAsBool` _returnvalue (`self.HasSeenPlayerName`) false)
    (else
      (cast `/Game/_GameJamLN2024/Blueprints/Player/BP_Character` Actor)
      (`KismetSystemLibrary.PrintString` "cannot see character")
      (`BlackboardComponent.SetValueAsBool` _returnvalue _canseeplayername false)
      (`BlackboardComponent.SetValueAsBool` _returnvalue (`self.HasSeenPlayerName`) true)
      (`BlackboardComponent.SetValueAsVector` _returnvalue (`self.LastSeenPlayerLocationName`) Stimulus_StimulusLocation))))

(event `self.CapsuleComponent.OnComponentHit`
  (params (HitComponent :type "PrimitiveComponent Object Reference") (OtherActor :type "Actor Object Reference") (OtherComp :type "PrimitiveComponent Object Reference") (NormalImpulse :type "Vector Structure") (Hit :type "HitResult Structure (by ref)"))
  (cast `/Game/_GameJamLN2024/Blueprints/Player/BP_Character` OtherActor)
  (bind _asbp_game_mode (cast `/Game/_GameJamLN2024/Blueprints/BP_GameMode` (`GameplayStatics.GetGameMode`)))
  (`/Game/_GameJamLN2024/Blueprints/BP_GameMode.Reset` _asbp_game_mode))

(fn `Reset`
  (bind _returnvalue (`AIBlueprintHelperLibrary.GetBlackboard` (`AIBlueprintHelperLibrary.GetAIController` self)))
  (`self.K2_SetActorLocation` (`self.SearchAreaCenter`) false true)
  (`BlackboardComponent.SetValueAsBool` _returnvalue (`self.CanSeePlayerName`) false)
  (`BlackboardComponent.SetValueAsBool` _returnvalue (`self.HasSeenPlayerName`) false))

(fn `UserConstructionScript`
  (bind _output_get (set `self.SearchAreaCenter` (`self.K2_GetActorLocation`)))
  (`KismetSystemLibrary.DrawDebugCircle` _output_get (`self.SearchRadius`) 20 (struct :`R` 1.0 :`G` 0.761808 :`B` 0.159794 :`A` 1.0) 0.1 10.0 (1.0 0.0 0.0) (0.0 1.0 0.0))
  (`KismetSystemLibrary.DrawDebugCircle` _output_get (+ (`self.SearchRadius`) (`self.FollowPlayerMaxRadius`)) 20 (struct :`R` 1.0 :`G` 0.016184 :`A` 1.0) 0.1 10.0 (1.0 0.0 0.0) (0.0 1.0 0.0)))