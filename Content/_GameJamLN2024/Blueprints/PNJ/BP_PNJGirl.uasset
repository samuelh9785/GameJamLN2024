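; BP_PNJGirl is an NPC that becomes happy once enough projectile hits land on its paint area.
; Each BP_Projectile overlap on AreaToPaintCollision increments a counter, and reaching the threshold sets IsHappy on the AI controller's Blackboard.
; Reset clears the counter and happy state, then teleports the NPC to the location saved at BeginPlay.
; Its capsule ignores the player character when moving.
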(event `self.ReceiveBeginPlay`
  (`PrimitiveComponent.IgnoreActorWhenMoving` (`self.CapsuleComponent`) (`GameplayStatics.GetPlayerCharacter` 0) true)
  (set `self.DefaultPos` (`self.K2_GetActorLocation`)))

(event `self.AreaToPaintCollision.OnComponentBeginOverlap`
  (params (OverlappedComponent :type "PrimitiveComponent Object Reference") (OtherActor :type "Actor Object Reference") (OtherComp :type "PrimitiveComponent Object Reference") (OtherBodyIndex :type Integer) (bFromSweep :type Boolean) (SweepResult :type "HitResult Structure (by ref)"))
  (cast `/Game/_GameJamLN2024/Blueprints/BP_Projectile` OtherActor)
  (bind _result (`/Engine/EditorBlueprintResources/StandardMacros.IncrementInt` (`self.ColoredAreaNumber`))
    (:`  `
      (bind _output_get (set `self.ColoredAreaNumber` _result))
      (if (>= _output_get (`self.NeedToColor`))
        (set `self.IsHappy` true)
        (`BlackboardComponent.SetValueAsBool` (`AIBlueprintHelperLibrary.GetBlackboard` (`AIBlueprintHelperLibrary.GetAIController` self)) (`self.IsHappyName`) (`self.IsHappy`))))))

(fn `Reset`
  (set `self.IsHappy` false)
  (`BlackboardComponent.SetValueAsBool` (`AIBlueprintHelperLibrary.GetBlackboard` (`AIBlueprintHelperLibrary.GetAIController` self)) (`self.IsHappyName`) (`self.IsHappy`))
  (set `self.ColoredAreaNumber` 0)
  (`self.K2_SetActorLocation` (`self.DefaultPos`) false true))

(fn `UserConstructionScript`)