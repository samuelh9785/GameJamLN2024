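; BP_GameMode is the game mode for a game jam project, handling checkpoint tracking and world reset.
; UpdateCheckpoint stores the current checkpoint on the game mode.
; Reset runs in sequence, calling Reset on every BP_Ennemy, then every BP_PNJ, then the player's BP_Character.
; Actors are gathered by class at reset time, and each one handles its own reset logic.
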(fn `Reset`
  (`|ExecutionSequence`
    (:`then_0`
      (bind _outactors (`GameplayStatics.GetAllActorsOfClass` "/Game/_GameJamLN2024/Blueprints/Ennemy/BP_Ennemy.BP_Ennemy_C"))
      (for _array_element _outactors
        (`/Game/_GameJamLN2024/Blueprints/Ennemy/BP_Ennemy.Reset` _array_element)))
    (:`then_1`
      (bind _outactors_2 (`GameplayStatics.GetAllActorsOfClass` "/Game/_GameJamLN2024/Blueprints/PNJ/BP_PNJ.BP_PNJ_C"))
      (for _array_element_2 _outactors_2
        (`/Game/_GameJamLN2024/Blueprints/PNJ/BP_PNJ.Reset` _array_element_2)))
    (:`then_2`
      (bind _asbp_character (cast `/Game/_GameJamLN2024/Blueprints/Player/BP_Character` (`GameplayStatics.GetPlayerCharacter` 0)))
      (`/Game/_GameJamLN2024/Blueprints/Player/BP_Character.Reset` _asbp_character))))

(fn `UpdateCheckpoint`
  (params (CurrentCheckpoint :type "/Game/_GameJamLN2024/Blueprints/Player/BP_Checkpoint Object Reference"))
  (set `self.CurrentCheckpoint` CurrentCheckpoint))

(fn `UserConstructionScript`)