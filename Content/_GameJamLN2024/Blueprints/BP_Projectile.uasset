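; BP_Projectile is a projectile that arcs to a supplied hit location and leaves a decal there.
; InitProjectile derives travel time from distance and starts a looping timer that moves it along a quadratic Bezier curve, built from nested lerps through a raised midpoint.
; On completion it spawns the decal facing along the hit normal, registers it in BP_GameMode's DecalList, sets its material's CenterPosition and destroys itself.
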(event `InitProjectile`
  (params (DecalMaterial :type "MaterialInstance Object Reference") (Hit :type "HitResult Structure"))
  (bind _returnvalue (`KismetMathLibrary.Vector_Distance` (`self.StartPos`) (`self.EndPos`)))
  (set `self.Decal Material` DecalMaterial)
  (set `self.StartPos` (`self.K2_GetActorLocation`))
  (set `self.EndPos` (`.Location` (`GameplayStatics.BreakHitResult` Hit)))
  (set `self.Distance` _returnvalue)
  (set `self.MidPos` (+ (`self.StartPos`) (* (`KismetMathLibrary.Normal` (- (`self.EndPos`) (`self.StartPos`))) (/ _returnvalue 2.0)) (0.0 0.0 200.0)))
  (set `self.MaxTime` (/ (`self.Distance`) (`self.SpeedFactor`)))
  (bind _returnvalue_2 (`KismetSystemLibrary.K2_SetTimerDelegate` (delegate `MoveProjectile`) 0.015 true))
  (set `self.Timer` _returnvalue_2))

(event `MoveProjectile`
  (bind _returnvalue (`self.K2_GetActorLocation`))
  (bind _decalsize (`self.DecalSize`))
  ;[1 1 1] Timer
  (bind _output_get (set `self.CurrentTime` (+ (`self.CurrentTime`) (`KismetSystemLibrary.K2_GetTimerElapsedTimeHandle` (`self.Timer`)))))
  (if (< _output_get (`self.MaxTime`))
    (`SceneComponent.K2_SetWorldLocation` (`self.DefaultSceneRoot`) (`self.LerpQuadratic` (`self.StartPos`) (`self.MidPos`) (`self.EndPos`) (/ (`self.CurrentTime`) (`self.MaxTime`))) false false)
    (else
      (`KismetSystemLibrary.K2_ClearAndInvalidateTimerHandle` (`self.Timer`))
      (bind _returnvalue_2 (`GameplayStatics.SpawnDecalAtLocation` (`self.Decal Material`) (`KismetMathLibrary.MakeVector` _decalsize _decalsize _decalsize) _returnvalue (`KismetMathLibrary.FindLookAtRotation` _returnvalue (+ _returnvalue (`.Normal` (`GameplayStatics.BreakHitResult` (stale `InitProjectile` Hit)))))))
      (bind _asbp_game_mode (cast `/Game/_GameJamLN2024/Blueprints/BP_GameMode` (`GameplayStatics.GetGameMode`)))
      (`KismetArrayLibrary.Array_Add` (`/Game/_GameJamLN2024/Blueprints/BP_GameMode.DecalList` _asbp_game_mode) _returnvalue_2)
      (bind _returnvalue_3 (`DecalComponent.CreateDynamicMaterialInstance` _returnvalue_2))
      (`MaterialInstanceDynamic.SetVectorParameterValue` _returnvalue_3 "CenterPosition" (`KismetMathLibrary.MakeColor` (.x (`self.GetActorBounds` false)) (.y (`self.GetActorBounds` false)) (.z (`self.GetActorBounds` false))))
      (`self.K2_DestroyActor`))))

(fn `LerpQuadratic`
  (params (Vector1 :type "Vector Structure") (Vector2 :type "Vector Structure") (Vector3 :type "Vector Structure") (Alpha :type "Float (double-precision)"))
  (returns (FinalVector :type "Vector Structure"))
  (bind _vector2 (`local.Vector2`))
  (return (`|EaseFunction` "Linear" (`local.Alpha`) (`|EaseFunction` "Linear" (`local.Alpha`) (`local.Vector1`) _vector2) (`|EaseFunction` "Linear" (`local.Alpha`) _vector2 (`local.Vector3`)))))

(fn `UserConstructionScript`)